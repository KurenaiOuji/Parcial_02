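; Turret actor that turns toward the player when it sees them and fires bullets.
; BeginPlay caches player pawn 0 as a BP_Player reference.
; When PawnSensing sees a BP_Player, the turret sets its yaw to face the cached player, then waits on a short Delay before spawning a BP_Turret_Bullet at ShottingPoint.
; The Delay ignores retriggers while pending, so it also throttles the fire rate.
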(event `self.ReceiveBeginPlay`
  (bind _asbp_player (cast `/Game/Blueprints/Character/BP_Player` (`GameplayStatics.GetPlayerPawn` 0)))
  (set `self.Player` _asbp_player))

(event `self.PawnSensing.OnSeePawn`
  (params (Pawn :type "Pawn Object Reference"))
  (bind (_returnvalue_roll _returnvalue_pitch _returnvalue_yaw) (`KismetMathLibrary.BreakRotator` (`KismetMathLibrary.FindLookAtRotation` (`self.K2_GetActorLocation`) (`self.K2_GetActorLocation` (`self.Player`)))))
  (cast `/Game/Blueprints/Character/BP_Player` Pawn)
  (`self.K2_SetActorRotation` (`KismetMathLibrary.MakeRotator` 0.0 0.0 _returnvalue_yaw))
  (`KismetSystemLibrary.Delay` 0.5)
  (`|SpawnActorFromClass` "/Game/Blueprints/Turret/BP_Turret_Bullet.BP_Turret_Bullet_C" (`SceneComponent.K2_GetComponentToWorld` (`self.Shotting_Point`)) "Undefined" "MultiplyWithRoot" null null))

(fn `UserConstructionScript`)